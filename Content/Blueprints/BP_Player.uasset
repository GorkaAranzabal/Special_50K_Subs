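; Player Blueprint that handles basic movement, camera look and jumping through Enhanced Input.
; BeginPlay adds the IMC_PlayerInput mapping context for player controller 0.
; Move input follows the full control rotation with the sideways axis negated, while look input drives controller yaw and inverted pitch.
; Jump fires on the action's Completed event, with no matching StopJumping call.
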(event `self.ReceiveBeginPlay`
  ;[0.0816 0.0816 0.0816] Input and Movement
  (`EnhancedInputSubsystemInterface.AddMappingContext` (pcsubsystem `EnhancedInputLocalPlayerSubsystem` (`GameplayStatics.GetPlayerController` 0)) "/Game/Input/IMC_PlayerInput.IMC_PlayerInput" 0 (struct)))

(event `EnhancedInput|/Game/Input/IA_Move`
  (params (ActionValue :type "Vector2D Structure") (ElapsedSeconds :type "Float (double-precision)") (TriggeredSeconds :type "Float (double-precision)") (InputAction :type "InputAction Object Reference" :default "/Game/Input/IA_Move.IA_Move"))
  ;[0.0816 0.0816 0.0816] Input and Movement
  (:`Triggered`
    (`self.AddMovementInput` (`KismetMathLibrary.GetForwardVector` (`self.GetControlRotation`)) ActionValue_Y)
    (`self.AddMovementInput` (`KismetMathLibrary.GetRightVector` (`self.GetControlRotation`)) (* ActionValue_X -1.0))))

(event `EnhancedInput|/Game/Input/IA_Look`
  (params (ActionValue :type "Vector2D Structure") (ElapsedSeconds :type "Float (double-precision)") (TriggeredSeconds :type "Float (double-precision)") (InputAction :type "InputAction Object Reference" :default "/Game/Input/IA_Look.IA_Look"))
  ;[0.0816 0.0816 0.0816] Input and Movement
  (:`Triggered`
    (`self.AddControllerPitchInput` (* ActionValue_Y -1.0))
    (`self.AddControllerYawInput` ActionValue_X)))

(event `EnhancedInput|/Game/Input/IA_Jump`
  (params (ActionValue :type Boolean) (ElapsedSeconds :type "Float (double-precision)") (TriggeredSeconds :type "Float (double-precision)") (InputAction :type "InputAction Object Reference" :default "/Game/Input/IA_Jump.IA_Jump"))
  ;[0.0816 0.0816 0.0816] Input and Movement
  (:`Completed`
    (`self.Jump`)))

(fn `UserConstructionScript`)