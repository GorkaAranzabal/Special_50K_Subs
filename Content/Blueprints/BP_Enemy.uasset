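; BP_Enemy is an enemy that roams randomly and is knocked out when the player hits it while falling.
; From BeginPlay, Wonder moves it via AIMoveTo to random reachable points nearby, pausing and repeating only after each successful move.
; DamageTrigger overlaps check for a falling BP_Player, then, only once, play a sound, halt movement and turn on mesh physics simulation.
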(event `self.ReceiveBeginPlay`
  (`self.Wonder`))

(event `Wonder`
  (`|AIMoveTo` self (`NavigationSystemV1.K2_GetRandomReachablePointInRadius` (`self.K2_GetActorLocation`) 5000.0 null null) null
    (:`OnSuccess`
      (`KismetSystemLibrary.Delay` 0.7)
      (`self.Wonder`))))

(event `self.Damage Trigger.OnComponentBeginOverlap`
  (params (OverlappedComponent :type "PrimitiveComponent Object Reference") (OtherActor :type "Actor Object Reference") (OtherComp :type "PrimitiveComponent Object Reference") (OtherBodyIndex :type Integer) (bFromSweep :type Boolean) (SweepResult :type "HitResult Structure (by ref)"))
  (if (`self.ActorHasTag` OtherActor "Player")
    (bind _asbp_player (cast `/Game/Blueprints/BP_Player` OtherActor))
    (if (`NavMovementComponent.IsFalling` (`Character.CharacterMovement` _asbp_player))
      (`/Engine/EditorBlueprintResources/StandardMacros.DoOnce` false
        (:`Completed`
          (`GameplayStatics.PlaySoundAtLocation` "/Engine/VREditor/Sounds/VR_teleport.VR_teleport" (`self.K2_GetActorLocation`) (struct) 1.0 1.0 0.0 "/Game/Audio/SA_Character.SA_Character" null null null)
          (`MovementComponent.StopMovementImmediately` (`self.CharacterMovement`))
          (`PrimitiveComponent.SetSimulatePhysics` (`self.Mesh`) true))))))

(fn `UserConstructionScript`)